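; BP_Player is the player Blueprint that handles the game's pause menu.
; On BeginPlay it creates the W_Pause widget once, adds it to the viewport and keeps it hidden.
; The Pause input toggles game pause, switching the widget's visibility, the mouse cursor and the input mode between Game Only and Game And UI.
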(event `self.ReceiveBeginPlay`
  ;[1 1 1] ポーズメニュー生成
  (`/Engine/EditorBlueprintResources/StandardMacros.IsValid` (`self.W_Pause`)
    (:`Is Not Valid`
      (bind _returnvalue (`|CreateWidget` "/Game/UI/W_Pause.W_Pause_C"))
      (bind _output_get (set `self.W_Pause` _returnvalue))
      (`UserWidget.AddToViewport` _output_get 1)
      (`Widget.SetVisibility` _output_get "Hidden"))))

(event `InputAction|Pause` :paused true
  (params (Key :type "Key Structure"))
  (bind _returnvalue (`GameplayStatics.GetPlayerController` 0))
  (bind _w_pause (`self.W_Pause`))
  ;[1 1 1] ポーズメニューの表示・非表示
  (:`Pressed`
    (if (`GameplayStatics.IsGamePaused`)
      (`GameplayStatics.SetGamePaused` false)
      (`Widget.SetVisibility` _w_pause "Hidden")
      (set `PlayerController.bShowMouseCursor` false _returnvalue)
      (`WidgetBlueprintLibrary.SetInputMode_GameOnly` _returnvalue)
      (else
        (`GameplayStatics.SetGamePaused` true)
        (`Widget.SetVisibility` _w_pause "Visible")
        (set `PlayerController.bShowMouseCursor` true _returnvalue)
        (`WidgetBlueprintLibrary.SetInputMode_GameAndUIEx` _returnvalue null)))))

(fn `UserConstructionScript`)